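; Two-way teleport actor that moves the first-person character between an inside and an outside destination, with a plane showing a render texture.
; BeginPlay builds a dynamic material from the mirror camera material, feeds it the render texture and applies it to the plane.
; Box overlap reads the character's IsInside flag to pick the destination, moves it there, then flips the flag.
; A timeline-based delayed teleport is left unconnected.
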(event OnComponentBeginOverlap(Box)
  (params (OverlappedComponent :type Primitive%20Component%20Object%20Reference) (OtherActor :type Actor%20Object%20Reference) (OtherComp :type Primitive%20Component%20Object%20Reference) (OtherBodyIndex :type Integer) (bFromSweep :type Boolean) (SweepResult :type Hit%20Result%20Structure%20%28by%20ref%29))
  ;[0.5599 1 0.5568] Teleport
  (bind _asbp_first_person_character (Utilities|Casting|CastToBP_FirstPersonCharacter OtherActor))
  (if (Variables|/Game/FirstPerson/Blueprints/BP_FirstPersonCharacter.BP_FirstPersonCharacter_C|GetIsInside _asbp_first_person_character)
    (Transformation|SetActorLocation OtherActor (Transformation|GetActorLocation (Variables|Default|GetTeleportOutside)) false false)
    (else
      (Transformation|SetActorLocation OtherActor (Transformation|GetActorLocation (Variables|Default|GetTeleportInside)) false false)))
  (Variables|/Game/FirstPerson/Blueprints/BP_FirstPersonCharacter.BP_FirstPersonCharacter_C|SetIsInside _asbp_first_person_character (not (Variables|/Game/FirstPerson/Blueprints/BP_FirstPersonCharacter.BP_FirstPersonCharacter_C|GetIsInside _asbp_first_person_character))))

(event EventBeginPlay
  ;[0.4323 0.6575 1] Create the Material for the teleport
  (bind _returnvalue (Rendering|Material|CreateDynamicMaterialInstance "/Game/NonEuclideanAssets/Materials/MirrorCameraMaterial.MirrorCameraMaterial" "None" "None" :!class /Script/Engine.KismetMaterialLibrary))
  (bind _output_get (Variables|Default|SetMaterial _returnvalue))
  (Rendering|Material|SetTextureParameterValue _output_get "MirrorTexture" (Variables|Default|GetRender))
  (Rendering|Material|SetMaterial (Variables|Default|GetPlane) 0 (Variables|Default|GetMaterial)))

(event Collision|EventActorBeginOverlap
  (params (OtherActor :type Actor%20Object%20Reference)))

(event EventTick
  (params (DeltaSeconds :type Float%20%28single-precision%29)))

(fn ConstructionScript)