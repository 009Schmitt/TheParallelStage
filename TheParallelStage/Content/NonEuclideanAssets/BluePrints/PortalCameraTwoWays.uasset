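; Portal camera actor for a two-way portal that turns to match the player's viewing angle and flips the portal surface.
; Each tick it computes a look-at yaw from the referenced Portal toward the player pawn and applies it to itself.
; When that yaw lies strictly within ±90 degrees and the first-person character is not flagged IsInside, the Portal turns 180 degrees from its BeginPlay yaw; otherwise it keeps that yaw.
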(event EventBeginPlay
  ;[0.6678 1 0.4152] Setup StartRotation
  (Variables|Default|SetStartRotation (.yaw (Transformation|GetActorRotation (Variables|Default|GetPortal)))))

(event Collision|EventActorBeginOverlap
  (params (OtherActor :type Actor%20Object%20Reference)))

(event EventTick
  (params (DeltaSeconds :type Float%20%28single-precision%29))
  (bind _returnvalue (Game|Player|GetPlayerPawn 0))
  (bind _portal (Variables|Default|GetPortal))
  (bind _returnvalue_2 (Transformation|GetActorLocation _returnvalue))
  (bind _rootcomponent (Variables|/Script/Engine.Actor|GetRootComponent _portal))
  (bind _returnvalue_3 (Transformation|GetWorldTransform _rootcomponent))
  (bind _returnvalue_4 (Transformation|GetWorldTransform _rootcomponent))
  (bind _returnvalue_5 (Components|GetChildComponent _rootcomponent 1))
  (bind _returnvalue_6 (Math|Vector|GetForwardVector _returnvalue_5))
  (bind _returnvalue_7 (Math|Transform|InverseTransformDirection _returnvalue_3 _returnvalue_6))
  (bind _returnvalue_8 (Class|KismetAnimationLibrary|Lookat _returnvalue_4 _returnvalue_2 _returnvalue_7 true "0, 0, 0" 0.0))
  ;[1 0.6349 0.473] Camera Angle
  (Transformation|SetActorRotation self (Math|Rotator|MakeRotator 0.0 0.0 (.yaw (.rotation _returnvalue_8))))
  ;[0.8515 1 0.3604] Flipping Mechanic
  (bind _asbp_first_person_character (Utilities|Casting|CastToBP_FirstPersonCharacter (Game|Player|GetPlayerPawn 0)))
  (if (or (Variables|/Game/FirstPerson/Blueprints/BP_FirstPersonCharacter.BP_FirstPersonCharacter_C|GetIsInside _asbp_first_person_character) (or (>= (.yaw (.rotation _returnvalue_8)) 9e+01) (<= (.yaw (.rotation _returnvalue_8)) -9e+01)))
    (Variables|Default|SetisFlipped false)
    (else
      (Variables|Default|SetisFlipped true)))
  (if (Variables|Default|GetisFlipped)
    (Transformation|SetActorRotation (Variables|Default|GetPortal) (Math|Rotator|MakeRotator 9e+01 0.0 (+ (Variables|Default|GetStartRotation) 1.8e+02)))
    (else
      (Transformation|SetActorRotation (Variables|Default|GetPortal) (Math|Rotator|MakeRotator 9e+01 0.0 (Variables|Default|GetStartRotation))))))

(fn ConstructionScript)