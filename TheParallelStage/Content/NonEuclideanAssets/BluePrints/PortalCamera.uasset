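; PortalCamera is an actor Blueprint that sets its viewing angle from the player's position relative to a referenced Portal.
; Each Tick, it runs LookAt from the Portal's root transform toward the player pawn, using the forward vector of one of the Portal's child components, converted to local space, as the aim axis.
; Only the resulting yaw feeds the actor's rotation, so the camera turns horizontally.
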(event EventBeginPlay)

(event Collision|EventActorBeginOverlap
  (params (OtherActor :type Actor%20Object%20Reference)))

(event EventTick
  (params (DeltaSeconds :type Float%20%28single-precision%29))
  (bind _portal (Variables|Default|GetPortal))
  (bind _rootcomponent (Variables|/Script/Engine.Actor|GetRootComponent _portal))
  ;[1 0.6349 0.473] Camera Angle
  (Transformation|SetActorRotation self (Math|Rotator|MakeRotator 0.0 0.0 (.yaw (.rotation (Class|KismetAnimationLibrary|Lookat (Transformation|GetWorldTransform _rootcomponent) (Transformation|GetActorLocation (Game|Player|GetPlayerPawn 0)) (Math|Transform|InverseTransformDirection (Transformation|GetWorldTransform _rootcomponent) (Math|Vector|GetForwardVector (Components|GetChildComponent _rootcomponent 1))) true "0, 0, 0" 0.0))))))

(fn ConstructionScript)