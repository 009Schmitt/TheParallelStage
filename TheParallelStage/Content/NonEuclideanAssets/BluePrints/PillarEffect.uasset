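; Non-Euclidean pillar actor that swaps its Object mesh through MeshList as overlaps hit its trigger volumes, apparently as the player circles it.
; Plus steps to the next mesh and Minus to the previous, wrapping at the list ends.
; Two flags block repeat steps from the same trigger.
; MidArea, marking a front pass, sets both flags so the next Plus or Minus overlap only clears them.
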(event OnComponentBeginOverlap(Minus)
  (params (OverlappedComponent :type Primitive%20Component%20Object%20Reference) (OtherActor :type Actor%20Object%20Reference) (OtherComp :type Primitive%20Component%20Object%20Reference) (OtherBodyIndex :type Integer) (bFromSweep :type Boolean) (SweepResult :type Hit%20Result%20Structure%20%28by%20ref%29))
  ;[0.9421 1 0.4542] Previous Mesh
  (if (Variables|Default|GetMinusHappened)
    (if (Variables|Default|GetPlusHappened)
      (Variables|Default|SetMinusHappened false)
      (Variables|Default|SetPlusHappened false))
    (else
      (bind _result (Math|Integer|DecrementInt (Variables|Default|GetMeshIndex))
        (:%20%20
          (if (< _result 0)
            (bind _result_2 (Math|Integer|DecrementInt (Utilities|Array|Length (Variables|Default|GetMeshList)))
              (:%20%20
                (Variables|Default|SetMeshIndex _result_2))))
          (Components|StaticMesh|SetStaticMesh (Variables|Default|GetObject) (Utilities|Array|Get(acopy) (Variables|Default|GetMeshList) (Variables|Default|GetMeshIndex)))
          (Variables|Default|SetMinusHappened true)
          (Variables|Default|SetPlusHappened false))))))

(event OnComponentBeginOverlap(Plus)
  (params (OverlappedComponent :type Primitive%20Component%20Object%20Reference) (OtherActor :type Actor%20Object%20Reference) (OtherComp :type Primitive%20Component%20Object%20Reference) (OtherBodyIndex :type Integer) (bFromSweep :type Boolean) (SweepResult :type Hit%20Result%20Structure%20%28by%20ref%29))
  ;[0.9617 1 0.4084] Next Mesh
  (if (Variables|Default|GetPlusHappened)
    (if (Variables|Default|GetMinusHappened)
      (Variables|Default|SetMinusHappened false)
      (Variables|Default|SetPlusHappened false))
    (else
      (bind _result (Math|Integer|IncrementInt (Variables|Default|GetMeshIndex))
        (:%20%20
          (if (== _result (Utilities|Array|Length (Variables|Default|GetMeshList)))
            (Variables|Default|SetMeshIndex 0))
          (Components|StaticMesh|SetStaticMesh (Variables|Default|GetObject) (Utilities|Array|Get(acopy) (Variables|Default|GetMeshList) (Variables|Default|GetMeshIndex)))
          (Variables|Default|SetPlusHappened true)
          (Variables|Default|SetMinusHappened false))))))

(event OnComponentBeginOverlap(MidArea)
  (params (OverlappedComponent :type Primitive%20Component%20Object%20Reference) (OtherActor :type Actor%20Object%20Reference) (OtherComp :type Primitive%20Component%20Object%20Reference) (OtherBodyIndex :type Integer) (bFromSweep :type Boolean) (SweepResult :type Hit%20Result%20Structure%20%28by%20ref%29))
  ;[0.9247 1 0.4623] Confer if player passed through the front
  (Variables|Default|SetMinusHappened true)
  (Variables|Default|SetPlusHappened true))

(event EventBeginPlay
  ;[0.969 1 0.3804] Set a Start Mesh
  (Components|StaticMesh|SetStaticMesh (Variables|Default|GetObject) (Utilities|Array|Get(acopy) (Variables|Default|GetMeshList))))

(event Collision|EventActorBeginOverlap
  (params (OtherActor :type Actor%20Object%20Reference)))

(event EventTick
  (params (DeltaSeconds :type Float%20%28single-precision%29)))

(fn ConstructionScript)